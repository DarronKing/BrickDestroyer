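; VR_PawnTest is a test VR pawn that equips both hands with BoardVRTest actors.
; On BeginPlay it spawns one owned BoardVRTest per side and stores them as RightController and LeftController.
; Each is attached to its MCRight or MCLeft component with keep-relative rules, so it follows that component.
; The pawn has no other graph logic.
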(event EventBeginPlay
  (bind _returnvalue (Math|Transform|MakeTransform "0, 0, 0"))
  (bind _self self)
  (Utilities|FlowControl|Sequence
    (:then_0
      (bind _returnvalue_2 (Game|SpawnActorfromClass "/Game/Blueprints/VR_Stuffs/BoardVRTest.BoardVRTest_C" _returnvalue "Undefined" _self 0))
      (Variables|Default|SetRightController _returnvalue_2)
      (Transformation|AttachComponentToComponent _returnvalue_2 (Variables|Default|GetMC_Right) "None" "KeepRelative" "KeepRelative" "KeepRelative" false))
    (:then_1
      (bind _returnvalue_3 (Game|SpawnActorfromClass "/Game/Blueprints/VR_Stuffs/BoardVRTest.BoardVRTest_C" _returnvalue "Undefined" _self 0))
      (Variables|Default|SetLeftController _returnvalue_3)
      (Transformation|AttachComponentToComponent _returnvalue_3 (Variables|Default|GetMC_Left) "None" "KeepRelative" "KeepRelative" "KeepRelative" false))))

(fn ConstructionScript)