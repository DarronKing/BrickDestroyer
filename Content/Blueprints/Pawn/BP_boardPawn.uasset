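; BP_boardPawn is the player's board, moved vertically and horizontally by axis input, that collects powerups and applies them to bouncing balls.
; Overlapping a star, fuel can or repair powerup destroys it, changes the board's material and stores the type in an enum.
; On a ball hit, fuel can multiplies velocity and repair spawns another ball after a short delay, then the enum resets.
; The star's strength effect is an empty stub.
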(event OnComponentBeginOverlap(boardCollision)
  (params (OverlappedComponent :type Primitive%20Component%20Object%20Reference) (OtherActor :type Actor%20Object%20Reference) (OtherComp :type Primitive%20Component%20Object%20Reference) (OtherBodyIndex :type Integer) (bFromSweep :type Boolean) (SweepResult :type Hit%20Result%20Structure%20%28by%20ref%29))
  ;[1 1 1] Destroy Powerups
  (if (Utilities|ClassIsChildOf (Utilities|GetClass OtherActor) "/Game/Blueprints/Powerups/PowerupParent.PowerupParent_C")
    (Actor|DestroyActor OtherActor)
    ;[1 1 1] Apply Powerup To Board
    (if (Utilities|ClassIsChildOf (Utilities|GetClass OtherActor) "/Game/Blueprints/Powerups/StarPowerup.StarPowerup_C")
      (Rendering|Material|SetMaterial (Variables|Default|Getboard) 0 "/Game/Geometry/textures/powerUp_one.powerUp_one")
      (Variables|Default|SetPowerUpInteger 1)
      (Variables|Default|SetPowerupEnum "NewEnumerator0")
      (elif (Utilities|ClassIsChildOf (Utilities|GetClass OtherActor) "/Game/Blueprints/Powerups/FuelCanPowerup.FuelCanPowerup_C")
        (Rendering|Material|SetMaterial (Variables|Default|Getboard) 0 "/Game/Geometry/textures/powerUp_one.powerUp_one")
        (Variables|Default|SetPowerUpInteger 2)
        (Variables|Default|SetPowerupEnum "NewEnumerator2")
        (elif (Utilities|ClassIsChildOf (Utilities|GetClass OtherActor) "/Game/Blueprints/Powerups/RepairPowerup.RepairPowerup_C")
          (Rendering|Material|SetMaterial (Variables|Default|Getboard) 0 "/Game/Geometry/textures/powerUp_one.powerUp_one")
          (Variables|Default|SetPowerUpInteger 3)
          (Variables|Default|SetPowerupEnum "NewEnumerator1"))))))

(event Collision|EventHit
  (params (MyComp :type Primitive%20Component%20Object%20Reference) (Other :type Actor%20Object%20Reference) (OtherComp :type Primitive%20Component%20Object%20Reference) (bSelfMoved :type Boolean) (HitLocation :type Vector :default "0, 0, 0") (HitNormal :type Vector :default "0, 0, 0") (NormalImpulse :type Vector :default "0, 0, 0") (Hit :type Hit%20Result%20Structure%20%28by%20ref%29))
  ;[1 1 1] Apply Powerup To Ball
  (if (not (and (Utilities|ClassIsChildOf "/Game/Blueprints/BP_bouncingBall.BP_bouncingBall_C" (Utilities|GetClass Other)) (Utilities|Enum|Equal(Enum) (Variables|Default|GetPowerupEnum) "NewEnumerator0")))
    (if (and (Utilities|ClassIsChildOf "/Game/Blueprints/BP_bouncingBall.BP_bouncingBall_C" (Utilities|GetClass Other)) (Utilities|Enum|Equal(Enum) (Variables|Default|GetPowerupEnum) "NewEnumerator2"))
      (bind _asbp_bouncing_ball (Utilities|Casting|CastToBP_bouncingBall Other))
      (CallFunction|PUIncreaseSpeed _asbp_bouncing_ball)
      (Variables|Default|SetPowerupEnum "NewEnumerator4")
      (elif (and (Utilities|ClassIsChildOf "/Game/Blueprints/BP_bouncingBall.BP_bouncingBall_C" (Utilities|GetClass Other)) (Utilities|Enum|Equal(Enum) (Variables|Default|GetPowerupEnum) "NewEnumerator1"))
        (Utilities|FlowControl|Delay 0.2)
        (CallFunction|PUSplitBall)
        (Variables|Default|SetPowerupEnum "NewEnumerator4")))))

(event Input|AxisEvents|InputAxisboardHorizontalMovement
  (params (AxisValue :type Float%20%28single-precision%29))
  ;[1 1 1] Board Movement
  (Transformation|AddRelativeLocation (Variables|Default|GetboardCollision) (Math|Vector|MakeVector 0.0 AxisValue 0.0) false false))

(event Input|AxisEvents|InputAxisboardVerticalMovement
  (params (AxisValue :type Float%20%28single-precision%29))
  ;[1 1 1] Board Movement
  (Transformation|AddRelativeLocation (Variables|Default|GetboardCollision) (Math|Vector|MakeVector 0.0 0.0 AxisValue) false false))

(fn ConstructionScript)

(fn PUSplitBall
  (bind _returnvalue (Game|SpawnActorfromClass "/Game/Blueprints/BP_bouncingBall.BP_bouncingBall_C" (Math|Conversions|ToTransform(Vector) (Transformation|GetActorLocation)) "Undefined" 0 0))
  (Transformation|DetachFromActor _returnvalue "KeepWorld" "KeepWorld" "KeepWorld")
  (Default|SetVelocity _returnvalue "0, 0, 0"))

(fn PUIncreaseSpeed
  (params (Ball :type BP%20Bouncing%20Ball%20Object%20Reference))
  (bind _velocty (Default|GetVelocty Ball))
  (Default|SetVelocity Ball (* _velocty "1.500000,1.500000,1.500000"))
  (return))

(fn PUStrength)