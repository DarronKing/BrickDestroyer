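; Base Blueprint for powerups, which drift through the level for a limited time.
; On BeginPlay the Move timeline adds its MoveX output to the actor's location each update, and a Delay in that update chain destroys the actor ten seconds later.
; SendEnum appears meant for child overrides, as the parent version prints a warning and returns a fixed enum value.
; Overlap and hit events do nothing, leaving pawn-contact destruction unconnected.
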(event OnComponentHit(Box)
  (params (HitComponent :type Primitive%20Component%20Object%20Reference) (OtherActor :type Actor%20Object%20Reference) (OtherComp :type Primitive%20Component%20Object%20Reference) (NormalImpulse :type Vector :default "0, 0, 0") (Hit :type Hit%20Result%20Structure%20%28by%20ref%29)))

(event EventBeginPlay
  ;[1 1 1] Move Towards Death
  (bind _movex (Timeline|Move PlayFromStart)
    (:Update
      (Transformation|SetActorLocation (+ _movex (Transformation|GetActorLocation)) false false)
      (Utilities|FlowControl|Delay 1e+01)
      (Actor|DestroyActor))))

(event Collision|EventActorBeginOverlap
  (params (OtherActor :type Actor%20Object%20Reference)))

(event Collision|EventActorEndOverlap
  (params (OtherActor :type Actor%20Object%20Reference)))

(fn ConstructionScript)

(fn SendEnum
  (Development|PrintString "Oh no, parent somehow is in game.........")
  (return "NewEnumerator0"))