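; Parent brick Blueprint for a brick-breaker game: a breakable block that drops a power-up.
; On BeginPlay it registers with the bouncing ball's remaining-brick count and rolls random health.
; Each hit lowers health and updates the material, which is randomly picked at one health.
; At zero it decrements the count, destroys the hit component rather than the actor, and spawns a random power-up.
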(event OnComponentHit(brick)
  (params (HitComponent :type Primitive%20Component%20Object%20Reference) (OtherActor :type Actor%20Object%20Reference) (OtherComp :type Primitive%20Component%20Object%20Reference) (NormalImpulse :type Vector :default "0, 0, 0") (Hit :type Hit%20Result%20Structure%20%28by%20ref%29))
  (bind _health (Variables|Default|GetHealth))
  ;[1 1 1] minus health when hit
  (Math|Integer|DecrementInt _health
    (:%20%20
      ;[1 1 1] Destroy Brick if dead
      (if (<= _health 0)
        (Default|DecrimentBricksRemaingin (Variables|Default|GetBouncingBallRef))
        (Components|DestroyComponent HitComponent)
        ;[1 1 1] Spawn Powerup
        (bind _powerup (CallFunction|GetRandomPowerup (Variables|Default|GetPowerups)))
        (Game|SpawnActorfromClass _powerup (Math|Conversions|ToTransform(Vector) (Transformation|GetActorLocation)) "Undefined" 0 0)
        (else
          (CallFunction|ChangeTexture))))))

(event EventBeginPlay
  ;[1 1 1] Count Bricks
  (Default|IncrementBricksRemaining (Variables|Default|GetBouncingBallRef))
  (Variables|Default|SetHealth (Math|Random|RandomIntegerinRange 1 3))
  (CallFunction|ChangeTexture))

(fn ConstructionScript)

(fn DestroyBrick)

(fn GetRandomPowerup
  (params (PowerupArray :type Array%20of%20Powerup%20Parent%20Class%20References))
  (return (Utilities|Array|Get(acopy) PowerupArray (Math|Random|RandomInteger (Utilities|Array|Length PowerupArray)))))

(fn ChangeTexture
  (switch int (Variables|Default|GetHealth)
    (:1
      ;[1 1 1] 1 Health
      (bind _object (CallFunction|GetRandomMaterial (Variables|Default|GetMaterials)))
      (Rendering|Material|SetMaterial (Variables|Default|Getbrick) 0 _object)
      (return))
    (:2
      (Rendering|Material|SetMaterial (Variables|Default|Getbrick) 0 "/Game/VirtualReality/Materials/M_ArcEndpoint.M_ArcEndpoint"))
    (:3
      (Rendering|Material|SetMaterial (Variables|Default|Getbrick) 0 "/Game/VirtualReality/Materials/MI_BaseMaterial3.MI_BaseMaterial3"))))

(fn GetRandomMaterial
  (params (Array :type Array%20of%20Material%20Interface%20Object%20References))
  (return (Utilities|Array|Get(acopy) Array (Math|Random|RandomInteger (Utilities|Array|Length Array)))))